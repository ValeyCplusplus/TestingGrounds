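; AI controller Blueprint for guard NPCs that senses targets and passes them to a behavior tree.
; On BeginPlay it sets up the PatrolData blackboard and runs the GuardBehave tree.
; AI Perception updates store any sensed actor without the "NPC" tag under EnemyKey, and clear that key when such an actor's stimulus is not successfully sensed.
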(event `self.ReceiveBeginPlay`
  (bind _blackboardcomponent (`self.UseBlackboard` "/Game/AI/PatrolData.PatrolData"))
  (set `self.BlackboardC` _blackboardcomponent)
  (`self.RunBehaviorTree` "/Game/AI/GuardBehave.GuardBehave"))

(event `self.AIPerception.OnTargetPerceptionUpdated`
  (params (Actor :type "Actor Object Reference") (Stimulus :type "AIStimulus Structure"))
  (if (`self.ActorHasTag` Actor "NPC")
    _
    (elif (`.bSuccessfullySensed` (break `AIStimulus` Stimulus))
      (`BlackboardComponent.SetValueAsObject` (`self.BlackboardC`) (`self.EnemyKey`) Actor)
      (else
        (`BlackboardComponent.ClearValue` (`self.BlackboardC`) (`self.EnemyKey`))))))

(fn `UserConstructionScript`)